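; BP_Platform is a cart that carries the VR-style interaction pawn and control table between Head, Left Arm, Mid Arms and Right Arm stations.
; Arrow button presses pick an adjacent station from the last position, ignored while moving.
; Tick moves the cart at constant speed toward the mapped location, shifting attached actors by the same vector.
; On arrival within a distance buffer, it reports the new position to MechControl.
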(event `self.ReceiveBeginPlay`
  (bind _attachedactors (`self.AttachedActors`))
  (bind _returnvalue (`GameplayStatics.GetActorOfClass` "/Game/_MechaMove_Folder/BP_WorldInteractionPawn_Migrate.BP_WorldInteractionPawn_Migrate_C"))
  (`KismetArrayLibrary.Array_Add` _attachedactors _returnvalue)
  (bind _returnvalue_2 (`GameplayStatics.GetActorOfClass` "/Game/_MechaMove_Folder/Blueprints/BP_ControlTable.BP_ControlTable_C"))
  (`KismetArrayLibrary.Array_Add` _attachedactors _returnvalue_2)
  (bind _outactors (`GameplayStatics.GetAllActorsOfClass` "/Game/_MechaMove_Folder/Blueprints/BP_ArrowButton.BP_ArrowButton_C"))
  (for _array_element _outactors
    (add `/Game/_MechaMove_Folder/Blueprints/BP_ArrowButton.Pressed` _array_element (delegate `DPadPressed`))))

(event `DPadPressed`
  (params (Direction :type "/Game/_MechaMove_Folder/Blueprints/ButtonDirEnum Enum" :default "NewEnumerator0"))
  (`self.DPadInput` Direction))

(event `self.ReceiveTick`
  (params (DeltaSeconds :type "Float (single-precision)"))
  (bind _returnvalue (`self.K2_GetActorLocation`))
  (bind _value (`BlueprintMapLibrary.Map_Find` (`self.PositionMap`) (`self.Destination`)))
  (if (`|EnumEquality` (`self.Destination`) (`self.LastPosition`))
    _
    (elif (<= (`KismetMathLibrary.Vector_Distance` _value _returnvalue) (`self.PositionBuffer`))
      (`self.ArriveAtDestination`)
      (else
        (bind _output_get (set `self.MoveVector` (* (`KismetMathLibrary.Normal` (- _value _returnvalue)) (* DeltaSeconds (`self.MoveSpeed`)))))
        (`self.K2_SetActorLocation` (+ _output_get _returnvalue) :!pinned true) ; Moving the Cart
        (for _array_element (`self.AttachedActors`) :!pinned true
          (`self.K2_SetActorLocation` _array_element (+ (`self.K2_GetActorLocation` _array_element) (`self.MoveVector`)) false false))))))

(fn `ArriveAtDestination`
  (bind _output_get (set `self.LastPosition` (`self.Destination`)))
  (set `self.IsMoving` false)
  (`/Game/_MechaMove_Folder/Blueprints/BP_MechControl.UpdateCartPosition` (`|ConvertAsset` (`self.MechControl`)) _output_get))

(fn `DPadInput`
  (params (Direction :type "/Game/_MechaMove_Folder/Blueprints/ButtonDirEnum Enum" :default "NewEnumerator0"))
  (locals (PreDestination :type "/Game/_MechaMove_Folder/Blueprints/CartPosition Enum"))
  (bind _lastposition (`self.LastPosition`))
  (switch `/Game/_MechaMove_Folder/Blueprints/ButtonDirEnum` Direction
    (:`NewEnumerator0`
      (switch `/Game/_MechaMove_Folder/Blueprints/CartPosition` _lastposition
        (:`NewEnumerator2`
          (set `local.PreDestination` "NewEnumerator3"))))
    (:`NewEnumerator1`
      (switch `/Game/_MechaMove_Folder/Blueprints/CartPosition` _lastposition
        (:`NewEnumerator0`
          (set `local.PreDestination` "NewEnumerator2"))
        (:`NewEnumerator2`
          (set `local.PreDestination` "NewEnumerator1"))))
    (:`NewEnumerator2`
      (switch `/Game/_MechaMove_Folder/Blueprints/CartPosition` _lastposition
        (:`NewEnumerator3`
          (set `local.PreDestination` "NewEnumerator2"))))
    (:`NewEnumerator3`
      (switch `/Game/_MechaMove_Folder/Blueprints/CartPosition` _lastposition
        (:`NewEnumerator1`
          (set `local.PreDestination` "NewEnumerator2"))
        (:`NewEnumerator2`
          (set `local.PreDestination` "NewEnumerator0")))))
  (`self.NewDestination` (`local.PreDestination`)))

(fn `NewDestination`
  (params (Destination :type "/Game/_MechaMove_Folder/Blueprints/CartPosition Enum" :default "NewEnumerator0"))
  (if (not (`self.IsMoving`))
    (set `self.IsMoving` true)
    (set `self.Destination` Destination)))

(fn `UserConstructionScript`)