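; BP_MechControl is an actor meant as a mech control, linking a left and a right slider to mech movement, and is unfinished.
; On BeginPlay it binds a drag handler to each slider, but both handlers are empty.
; UpdateCartPosition is also an empty stub: its SetCartPosition call is disconnected, as is another in the event graph, and the MechMove reference is unused.
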(event `self.ReceiveBeginPlay`
  (add `/Game/ExampleContent/VR_World_Interaction/Blueprints/InteractiveObjects/BP_InteractiveSlider.SliderDraged` (`|ConvertAsset` (`self.LeftSlider`)) (delegate `LeftSliderDragged`))
  (add `/Game/ExampleContent/VR_World_Interaction/Blueprints/InteractiveObjects/BP_InteractiveSlider.SliderDraged` (`|ConvertAsset` (`self.RightSlider`)) (delegate `RightSliderDragged`)))

(event `LeftSliderDragged`
  (params (Position :type "Float (double-precision)")))

(event `RightSliderDragged`
  (params (Position :type "Float (double-precision)")))

(fn `UpdateCartPosition`
  (params (CartPosition :type "/Game/_MechaMove_Folder/Blueprints/CartPosition Enum" :default "NewEnumerator0")))

(fn `UserConstructionScript`)