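; BP_ArrowButton is a physically pushed arrow button that fires a Pressed event carrying its Direction, with hand feedback suggesting VR use.
; Tick converts the overlapping component's movement since first contact into clamped travel along the mesh's local Z, easing back when released.
; At full depth a DoOnce fires the event, sets the material's State parameter and, if an interactor is valid, plays feedback always on the left hand.
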(event `self.ReceiveTick`
  (params (DeltaSeconds :type "Float (single-precision)"))
  (bind _staticmeshcomponent (`self.StaticMeshComponent`))
  (bind (_returnvalue_x _returnvalue_y _returnvalue_z) (`KismetMathLibrary.BreakVector` (- (`KismetMathLibrary.InverseTransformDirection` (`SceneComponent.K2_GetComponentToWorld` _staticmeshcomponent) (`self.InitialOverlapLocation`)) (`KismetMathLibrary.InverseTransformDirection` (`SceneComponent.K2_GetComponentToWorld` _staticmeshcomponent) (`SceneComponent.K2_GetComponentLocation` (`self.OverlappedComponent`))))))
  (`/Engine/EditorBlueprintResources/StandardMacros.IsValid` (`self.OverlappedComponent`)
    (:`Is Valid`
      (bind _output_get (set `self.ButtonPressAmount` (`KismetMathLibrary.FClamp` _returnvalue_z 0.0 (`self.MaxButtonPress`))))
      (`SceneComponent.K2_SetRelativeLocation` (`self.StaticMeshComponent`) (- (`self.ButtonInitialLocation`) (`KismetMathLibrary.MakeVector` 0.0 0.0 _output_get)) false false)
      (if (>= (`self.ButtonPressAmount`) (`self.MaxButtonPress`))
        (`/Engine/EditorBlueprintResources/StandardMacros.DoOnce` false :!label _label
          (:`Completed`
            (`self.Pressed` (`self.Direction`))
            (`MeshComponent.SetScalarParameterValueOnMaterials` (`self.StaticMeshComponent`) "State" 1.0)
            (`/Engine/EditorBlueprintResources/StandardMacros.IsValid` (`self.CurrentInteractor`)
              (:`Is Valid`
                (`/Game/ExampleContent/VR_World_Interaction/Blueprints/FunctionLibraries/BPFL_FeedbackFunctionLibrary.PlayFeedbackOnHand` "Left" "NewEnumerator0" "NewEnumerator0" (`GameplayStatics.GetPlayerController` 0))))))
        (else
          (goto _label :!via `Reset`))))
    (:`Is Not Valid`
      (`SceneComponent.K2_SetRelativeLocation` (`self.StaticMeshComponent`) (`KismetMathLibrary.VInterpTo` (`SceneComponent.RelativeLocation` (`self.StaticMeshComponent`)) (`self.ButtonInitialLocation`) DeltaSeconds 10.0) false false))))

(event `self.StaticMeshComponent.OnComponentBeginOverlap`
  (params (OverlappedComponent :type "PrimitiveComponent Object Reference") (OtherActor :type "Actor Object Reference") (OtherComp :type "PrimitiveComponent Object Reference") (OtherBodyIndex :type Integer) (bFromSweep :type Boolean) (SweepResult :type "HitResult Structure (by ref)"))
  (`/Engine/EditorBlueprintResources/StandardMacros.IsValid` (`self.OverlappedComponent`)
    (:`Is Not Valid`
      (bind _output_get (set `self.OverlappedComponent` OtherComp))
      (set `self.InitialOverlapLocation` (`SceneComponent.K2_GetComponentLocation` _output_get)))))

(event `self.StaticMeshComponent.OnComponentEndOverlap`
  (params (OverlappedComponent :type "PrimitiveComponent Object Reference") (OtherActor :type "Actor Object Reference") (OtherComp :type "PrimitiveComponent Object Reference") (OtherBodyIndex :type Integer))
  (if (== OtherComp (`self.OverlappedComponent`))
    (set `self.OverlappedComponent` null)
    (`MeshComponent.SetScalarParameterValueOnMaterials` (`self.StaticMeshComponent`) "State" 0.0)))

(event `self.ReceiveBeginPlay`
  (set `self.ButtonInitialLocation` (`SceneComponent.RelativeLocation` (`self.StaticMeshComponent`))))

(fn `UserConstructionScript`)