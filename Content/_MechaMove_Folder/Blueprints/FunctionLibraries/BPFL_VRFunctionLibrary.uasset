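; Blueprint function library of VR helpers: headset type detection and quaternion math on a custom SQuat struct.
; GetHeadsetType maps the HMD device name to an enum, with a separate value when no HMD is enabled.
; Quaternion functions cover conjugate, negate, subtract, normalise, vector rotation and multiply, the last built from Math Expression nodes.
; RotatorToAxisAngle chains RotatorToQuat into QuatToAxisAngle, leaving an older inline conversion disconnected in its graph.
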(fn GetHeadsetType
  (if (Class|HeadMountedDisplayFunctionLibrary|IsHeadMountedDisplayEnabled)
    (switch name (Class|HeadMountedDisplayFunctionLibrary|GetHMDDeviceName)
      (:Default
        (return "NewEnumerator6"))
      (:SimpleHMD
        (return "NewEnumerator6"))
      (:OSVR
        (return "NewEnumerator4"))
      (:SteamVR
        (return "NewEnumerator2"))
      (:Unknown
        (return "NewEnumerator6"))
      (:GearVR
        (return "NewEnumerator3"))
      (:OculusRift
        (return "NewEnumerator1"))
      (:GoogleVR
        (return "NewEnumerator5")))
    (else
      (return "NewEnumerator0"))))

(fn RotatortoAxisAngle
  (params (Rotator :type Rotator))
  (bind _quat (CallFunction|RotatortoQuat Rotator))
  (bind (_axis _angle) (CallFunction|QuattoAxisAngle _quat))
  (return _axis _angle))

(fn RotatortoQuat
  (params (Rotator :type Rotator))
  (bind (_roll _pitch _yaw) (Math|Rotator|BreakRotator Rotator))
  (LocalVariables|SetDegToRadDiv2 (/ (/ (Math|Trig|GetPI) 1.8e+02) 2.0))
  (LocalVariables|Setsr (Math|Trig|Sin(Radians) (* _roll (LocalVariables|GetDegToRadDiv2))))
  (LocalVariables|Setcr (Math|Trig|Cos(Radians) (* _roll (LocalVariables|GetDegToRadDiv2))))
  (LocalVariables|Setsp (Math|Trig|Sin(Radians) (* _pitch (LocalVariables|GetDegToRadDiv2))))
  (LocalVariables|Setcp (Math|Trig|Cos(Radians) (* _pitch (LocalVariables|GetDegToRadDiv2))))
  (LocalVariables|Setsy (Math|Trig|Sin(Radians) (* _yaw (LocalVariables|GetDegToRadDiv2))))
  (LocalVariables|Setcy (Math|Trig|Cos(Radians) (* _yaw (LocalVariables|GetDegToRadDiv2))))
  (LocalVariables|Setw (+ (* (LocalVariables|Getcr) (LocalVariables|Getcp) (LocalVariables|Getcy)) (* (LocalVariables|Getsr) (LocalVariables|Getsp) (LocalVariables|Getsy))))
  (LocalVariables|Setx (- (* (LocalVariables|Getcr) (LocalVariables|Getsp) (LocalVariables|Getsy)) (* (LocalVariables|Getsr) (LocalVariables|Getcp) (LocalVariables|Getcy))))
  (LocalVariables|Sety (- (* -1.0 (LocalVariables|Getcr) (LocalVariables|Getsp) (LocalVariables|Getcy)) (* (LocalVariables|Getsr) (LocalVariables|Getcp) (LocalVariables|Getsy))))
  (LocalVariables|Setz (- (* (LocalVariables|Getcr) (LocalVariables|Getcp) (LocalVariables|Getsy)) (* (LocalVariables|Getsr) (LocalVariables|Getsp) (LocalVariables|Getcy))))
  (return (Utilities|Struct|MakeSQuat (LocalVariables|Getw) (LocalVariables|Getx) (LocalVariables|Gety) (LocalVariables|Getz))))

(fn QuatConjugate
  (params (In :type S%20Quat%20Structure))
  (bind (_w _x _y _z) (Utilities|Struct|BreakSQuat In))
  (return (Utilities|Struct|MakeSQuat _w (* _x -1.0) (* _y -1.0) (* _z -1.0))))

(fn QuatMultiply
  (params (A :type S%20Quat%20Structure) (B :type S%20Quat%20Structure))
  (bind (_w _x _y _z) (Utilities|Struct|BreakSQuat A))
  (bind (_w_2 _x_2 _y_2 _z_2) (Utilities|Struct|BreakSQuat B))
  (return (Utilities|Struct|MakeSQuat (|(((((neg1*x1)*x2)-(y1*y2))-(z1*z2))+(w1*w2)) -1.0 _x _x_2 _y _y_2 _z _z_2 _w _w_2) (|((((x1*w2)+(y1*z2))-(z1*y2))+(w1*x2)) _x _w_2 _y _z_2 _z _y_2 _w _x_2) (|(((((neg1*x1)*z2)+(y1*w2))+(z1*x2))+(w1*y2)) _x _z_2 _y -1.0 _w_2 _z _x_2 _w _y_2) (|((((x1*y2)-(y1*x2))+(z1*w2))+(w1*z2)) _x _y _y_2 _z _z_2 _w _w_2 _x_2))))

(fn QuatNegate
  (params (In :type S%20Quat%20Structure))
  (bind (_w _x _y _z) (Utilities|Struct|BreakSQuat In))
  (return (Utilities|Struct|MakeSQuat (* _w -1.0) (* _x -1.0) (* _y -1.0) (* _z -1.0))))

(fn QuattoAxisAngle
  (params (In :type S%20Quat%20Structure))
  (bind (_w _x _y _z) (Utilities|Struct|BreakSQuat In))
  (bind _output_get (LocalVariables|SetNorm (Math|Vector|MakeVector _x _y _z)))
  (bind _output_get_2 (LocalVariables|SetNorm (Math|Vector|Normalize _output_get)))
  (return _output_get_2 (* 2.0 (Math|Trig|Acos(Degrees) _w))))

(fn QuatSubtract
  (params (A :type S%20Quat%20Structure) (B :type S%20Quat%20Structure))
  (bind (_w _x _y _z) (Utilities|Struct|BreakSQuat A))
  (bind (_w_2 _x_2 _y_2 _z_2) (Utilities|Struct|BreakSQuat B))
  (return (Utilities|Struct|MakeSQuat (- _w _w_2) (- _x _x_2) (- _y _y_2) (- _z _z_2))))

(fn QuatNormalise
  (params (In :type S%20Quat%20Structure))
  (bind (_w _x _y _z) (Utilities|Struct|BreakSQuat In))
  (bind (_w_2 _x_2 _y_2 _z_2) (Utilities|Struct|BreakSQuat In))
  (bind _returnvalue (Math|Float|Square _x))
  (bind _returnvalue_2 (Math|Float|Square _w))
  (bind _returnvalue_3 (Math|Float|Square _y))
  (bind _returnvalue_4 (Math|Float|Square _z))
  (bind _returnvalue_5 (+ _returnvalue_2 _returnvalue _returnvalue_3 _returnvalue_4))
  (bind _returnvalue_6 (Math|Float|Sqrt _returnvalue_5))
  (return (select (== _returnvalue_6 0.0) (Utilities|Struct|MakeSQuat 1.0 0.0 0.0 0.0) (Utilities|Struct|MakeSQuat (/ _w_2 _returnvalue_6) (/ _x_2 _returnvalue_6) (/ _y_2 _returnvalue_6) (/ _z_2 _returnvalue_6)))))

(fn QuatMultiplyVector
  (params (A :type S%20Quat%20Structure) (B :type Vector))
  (bind (_w _x _y _z) (Utilities|Struct|BreakSQuat A))
  (bind _returnvalue (Math|Vector|MakeVector _x _y _z))
  (bind _returnvalue_2 (Math|Vector|CrossProduct _returnvalue B))
  (bind _returnvalue_3 (* _returnvalue_2 2.0))
  (return (+ B (* _returnvalue_3 _w) (Math|Vector|CrossProduct _returnvalue _returnvalue_3))))