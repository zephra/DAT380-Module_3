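; Fire altar actor whose flame particles, point light and fire sound are switched on or off together through SetFire.
; BeginPlay applies the initial FireOn state and binds TriggerFire to the EventHub trigger dispatcher, which toggles the fire after a TriggerName comparison.
; An endless random-delay loop from BeginPlay flickers the light intensity while FireOn is true; SetFire never updates that flag.
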(event `TriggerFire`
  (params (TriggerName :type String) (TriggerActive :type Boolean))
  ;[1 1 1] Triggering fire from trigger volume
  (if (`KismetStringLibrary.EqualEqual_StrStr` (`self.TriggerName`) TriggerName)
    (`self.SetFire` TriggerActive)))

(event `self.ReceiveBeginPlay`
  (bind _fireon (`self.FireOn`))
  ;[1 1 1] Basic setup
  (`self.SetFire` _fireon)
  (add `/Game/MYassets/Blueprints/EventHub.TriggerDispatcher` (`self.EventHub`) (delegate `TriggerFire`))
  ;[1 1 1] Fire flicker loop
  (`KismetSystemLibrary.Delay` (`KismetMathLibrary.RandomFloatInRange` 0.0 0.2) :!label _label)
  (if _fireon
    (`LightComponent.SetIntensity` (`self.PointLight`) (`KismetMathLibrary.RandomFloatInRange` 900.0 3000.0))
    (goto _label)
    (else
      (goto _label))))

(fn `SetFire`
  (params (FireActive :type Boolean))
  (`ActorComponent.SetActive` (`self.P_Fire`) FireActive false)
  (`SceneComponent.SetVisibility` (`self.PointLight`) FireActive false)
  (`ActorComponent.SetActive` (`self.Fire01_Cue`) FireActive false))

(fn `UserConstructionScript`)