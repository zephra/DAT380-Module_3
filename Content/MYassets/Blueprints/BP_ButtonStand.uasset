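; BP_ButtonStand is a pressable button on a statue stand that fires a named trigger when a motion controller touches it.
; Overlap by either hand controller, while no push is running, plays a timeline that slides the statue mesh from its starting position.
; A timeline event then calls CallTrigger on the level's EventHub with the configured name and active state, and plays a switch sound.
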(event `self.ReceiveBeginPlay`
  (set `self.ButtonInitialPosition` (`SceneComponent.RelativeLocation` (`self.SM_OniStatue02`)))
  (bind _returnvalue (`GameplayStatics.GetActorOfClass` "/Game/MYassets/Blueprints/EventHub.EventHub_C"))
  (set `self.EventHub` _returnvalue))

(event `self.ReceiveActorBeginOverlap`
  (params (OtherActor :type "Actor Object Reference"))
  (bind _returnvalue (`GameplayStatics.GetObjectClass` OtherActor))
  ;[1 1 1] Push buttton or not?
  (if (and (or (== _returnvalue "/Game/SjolieVRTemplates/VRCapablePawn/MotionController/BP_MotionController_Left.BP_MotionController_Left_C") (== _returnvalue "/Game/SjolieVRTemplates/VRCapablePawn/MotionController/BP_MotionController_Right.BP_MotionController_Right_C")) (not (`self.CurrentlyPushing`)))
    ;[1 1 1] Pushing animation
    (set `self.CurrentlyPushing` true)
    (bind (_direction _buttonpush) (`Timeline|Timeline_0` :!via `PlayFromStart`)
      (:`Update`
        (`SceneComponent.K2_SetRelativeLocation` (`self.SM_OniStatue02`) (+ _buttonpush (`self.ButtonInitialPosition`)) true false))
      (:`Finished`
        (set `self.CurrentlyPushing` false))
      (:`TriggerEvent`
        ;[1 1 1] Triggering events
        (`/Game/MYassets/Blueprints/EventHub.CallTrigger` (`self.EventHub`) (`self.TriggerName`) (`self.TriggerActive`))
        (`AudioComponent.Play` (`self.SwitchSound`) 0.0)))))

(fn `UserConstructionScript`)