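; BP_PickUp-able is a component that lets its owning actor be picked up and dropped.
; On BeginPlay it makes the owner's static mesh movable, physics-simulated and overlap-generating.
; Pickup turns off physics and attaches the owner's root to a supplied component, keeping its world transform.
; Drop restores physics and detaches the actor where it is.
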(event `self.ReceiveBeginPlay`
  (bind _output_get (set `self.Actor` (`self.GetOwner`)))
  (bind _returnvalue (`Actor.GetComponentByClass` _output_get "/Script/Engine.StaticMeshComponent"))
  (`SceneComponent.SetMobility` _returnvalue "Movable")
  (`PrimitiveComponent.SetSimulatePhysics` _returnvalue true)
  (set `PrimitiveComponent.bGenerateOverlapEvents` true _returnvalue))

(event `/Game/SjolieVRTemplates/EpicContent/VirtualRealityTemplate/Blueprints/PickupActorInterface.Pickup`
  (params (AttachTo :type "SceneComponent Object Reference"))
  (`PrimitiveComponent.SetSimulatePhysics` (`Actor.GetComponentByClass` (`self.Actor`) "/Script/Engine.StaticMeshComponent") false)
  (`SceneComponent.K2_AttachToComponent` (`Actor.K2_GetRootComponent` (`self.Actor`)) AttachTo "None" "KeepWorld" "KeepWorld" "KeepWorld" false))

(event `/Game/SjolieVRTemplates/EpicContent/VirtualRealityTemplate/Blueprints/PickupActorInterface.Drop`
  (`PrimitiveComponent.SetSimulatePhysics` (`Actor.GetComponentByClass` (`self.Actor`) "/Script/Engine.StaticMeshComponent") true)
  (`Actor.K2_DetachFromActor` (`self.Actor`) "KeepWorld" "KeepWorld" "KeepWorld"))